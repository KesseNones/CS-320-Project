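; ReplayBP is a timed test Blueprint that records gameplay and plays it back through the ReplayGameInstance.
; On BeginPlay, after a short delay, it starts recording, stops after a fixed interval and immediately starts the replay.
; On-screen messages mark the start and end of recording, and the game quits once a final playback delay elapses.
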(event EventBeginPlay
  (Utilities|FlowControl|Delay 2.0)
  (Development|PrintString "RECORDING" true true "(R=1.000000,G=0.039356,B=0.000000,A=1.000000)" 5.0)
  (bind _asreplay_game_instance (Utilities|Casting|CastToReplayGameInstance (Game|GetGameInstance)))
  (Class|ReplayGameInstance|StartRecord _asreplay_game_instance)
  (Utilities|FlowControl|Delay 2e+01)
  (Development|PrintString "STOP RECORDING" true true "(R=1.000000,G=0.039356,B=0.000000,A=1.000000)" 5.0)
  (bind _asreplay_game_instance_2 (Utilities|Casting|CastToReplayGameInstance (Game|GetGameInstance)))
  (Class|ReplayGameInstance|StopRecord _asreplay_game_instance_2)
  (bind _asreplay_game_instance_3 (Utilities|Casting|CastToReplayGameInstance (Game|GetGameInstance)))
  (Class|ReplayGameInstance|StartReplay _asreplay_game_instance_3)
  (Utilities|FlowControl|Delay 15.0)
  (Game|QuitGame 0 "Quit" false))

(fn ConstructionScript)